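; BP_Blocks is a grid of breakable blocks struck by BP_Ball, in what appears to be a brick-breaker game.
; The construction script adds one static mesh component per cell from X, Y and Padding.
; A ball hit switches an intact block to the cut-stone material, which doubles as its damage state.
; A hit on a cut-stone block spawns a random Bonus actor (weight 1.0) and destroys that component.
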(event EventBeginPlay)

(event Collision|EventActorBeginOverlap
  (params (OtherActor :type Actor%20Object%20Reference)))

(event Collision|EventHit
  (params (MyComp :type Primitive%20Component%20Object%20Reference) (Other :type Actor%20Object%20Reference) (OtherComp :type Primitive%20Component%20Object%20Reference) (bSelfMoved :type Boolean) (HitLocation :type Vector :default "0, 0, 0") (HitNormal :type Vector :default "0, 0, 0") (NormalImpulse :type Vector :default "0, 0, 0") (Hit :type Hit%20Result%20Structure%20%28by%20ref%29))
  (Utilities|Casting|CastToBP_Ball Other)
  (if (== (Rendering|Material|GetMaterial MyComp 0) "/Game/StarterContent/Materials/M_Brick_Cut_Stone.M_Brick_Cut_Stone")
    (Development|PrintString "Destroy" true true "(R=0.000000,G=1.000000,B=0.180039,A=1.000000)")
    (if (Math|Random|RandomBoolwithWeight 1.0)
      (Game|SpawnActorfromClass (.OutItem (Utilities|Array|Random (Variables|Default|GetBonus))) (Math|Transform|MakeTransform (Transformation|GetWorldLocation MyComp) "0.000000,50.000000,0.000000" "1.000000,1.000000,1.000000") "AlwaysSpawn" "MultiplyWithRoot" 0)
      (Components|DestroyComponent MyComp))
    (else
      (Development|PrintString "Material change" true true "(R=1.000000,G=0.133861,B=0.000000,A=1.000000)")
      (Rendering|Material|SetMaterial MyComp 0 "/Game/StarterContent/Materials/M_Brick_Cut_Stone.M_Brick_Cut_Stone"))))

(fn ConstructionScript
  (for _index (range 0 (Variables|SettingsBlock|GetX))
    (for _index_2 (range 0 (Variables|SettingsBlock|GetY))
      (AddComponent|AddStaticMeshComponent false (Math|Transform|MakeTransform (Math|Vector|MakeVector (Math|Conversions|ToFloat(Integer) (* _index (Variables|SettingsBlock|GetPadding))) (Math|Conversions|ToFloat(Integer) (* _index_2 (Variables|SettingsBlock|GetPadding))) 0.0))))))